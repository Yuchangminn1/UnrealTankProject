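; Tiger tank pawn Blueprint that drives the on-screen HUD for tank health and fire cooldown.
; BeginPlay creates both widgets, adds them to the viewport and seeds the HP widget from the Health value.
; Tick polls Health and mirrors the reload by counting LateCoolDown down from FireCoolDown while IsFireReady is false, sending -1 to the cooldown widget when ready.
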(event `self.ReceiveBeginPlay`
  (bind _returnvalue (`|CreateWidget` "/Game/Blueprints/Widgets/WBP_FireCoolDownWidget.WBP_FireCoolDownWidget_C"))
  (`UserWidget.AddToViewport` _returnvalue 0)
  (bind _returnvalue_2 (`|CreateWidget` "/Game/Blueprints/Widgets/WBP_TankHPWidget.WBP_TankHPWidget_C"))
  (`UserWidget.AddToViewport` _returnvalue_2 0)
  (set `/Game/Blueprints/Widgets/WBP_TankHPWidget.Health` (`HealthComponent.Health` (`self.Health`)) _returnvalue_2))

(event `self.ReceiveTick`
  (params (DeltaSeconds :type "Float (single-precision)"))
  (set `/Game/Blueprints/Widgets/WBP_TankHPWidget.Health` (`HealthComponent.Health` (`self.Health`)) (stale `self.ReceiveBeginPlay` _returnvalue_2))
  (if (`self.IsFireReady`)
    (set `/Game/Blueprints/Widgets/WBP_FireCoolDownWidget.Countdown` -1.0 (stale `self.ReceiveBeginPlay` _returnvalue))
    (set `self.LateCoolDown` (`self.FireCoolDown`))
    (else
      (bind _output_get (set `self.LateCoolDown` (- (`self.LateCoolDown`) DeltaSeconds)))
      (set `/Game/Blueprints/Widgets/WBP_FireCoolDownWidget.Countdown` _output_get (stale `self.ReceiveBeginPlay` _returnvalue)))))

(fn `UserConstructionScript`)